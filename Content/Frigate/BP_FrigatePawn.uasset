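; BP_FrigatePawn is the controllable pawn that steers a frigate and drives its orbit-style camera.
; On BeginPlay it destroys the Display child actor, spawns a separate BP_Frigate at its transform, attaches itself to it and passes on speed multipliers.
; Movement axes forward to that frigate, which is destroyed on EndPlay.
; BPPlayerCamera, configured with camera, spring arm and zoom limits in construction, handles look and frame-time-scaled zoom.
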(event `self.ReceiveBeginPlay`
  (`|ExecutionSequence`
    (:`then_0`
      (`self.K2_DestroyActor` (`ChildActorComponent.ChildActor` (`self.Display`)))
      (bind _returnvalue (`|SpawnActorFromClass` "/Game/Frigate/BP_Frigate.BP_Frigate_C" (`self.GetTransform`) "Undefined" "MultiplyWithRoot" null null))
      (bind _output_get (set `self.Frigate` _returnvalue))
      (`self.K2_AttachToActor` _output_get "None" "KeepWorld" "KeepWorld" "KeepWorld")
      (`/Game/Frigate/BP_Frigate.SetForwardSpeedMulti` _output_get (`self.FrigateForwardSpeed`))
      (`/Game/Frigate/BP_Frigate.SetRightSpeedMulti` _output_get (`self.FrigateRightSpeed`)))))

(event `self.ReceiveEndPlay`
  (params (EndPlayReason :type "EEndPlayReason Enum" :default "Destroyed"))
  (`self.K2_DestroyActor` (`self.Frigate`)))

(event `InputAxis|MoveForward`
  (params (AxisValue :type "Float (single-precision)"))
  (`/Game/Frigate/BP_Frigate.MoveForward` (`self.Frigate`) AxisValue))

(event `InputAxis|MoveRight`
  (params (AxisValue :type "Float (single-precision)"))
  (`/Game/Frigate/BP_Frigate.MoveRight` (`self.Frigate`) AxisValue))

(event `InputAxis|CameraUp`
  (params (AxisValue :type "Float (single-precision)"))
  (`/Game/Frigate/BP_PlayerCamera.AddUp` (`self.BP_PlayerCamera`) AxisValue))

(event `InputAxis|CameraRight`
  (params (AxisValue :type "Float (single-precision)"))
  (`/Game/Frigate/BP_PlayerCamera.AddRight` (`self.BP_PlayerCamera`) AxisValue))

(event `InputAxis|CameraZoom`
  (params (AxisValue :type "Float (single-precision)"))
  (`/Game/Frigate/BP_PlayerCamera.AddLength` (`self.BP_PlayerCamera`) (* AxisValue (`self.ZoomSpeedCore`) (`GameplayStatics.GetWorldDeltaSeconds`) (`self.ZoomSpeed`))))

(fn `UserConstructionScript`
  (bind _bp_playercamera (`self.BP_PlayerCamera`))
  (`/Game/Frigate/BP_PlayerCamera.SetCamera` _bp_playercamera (`self.Camera1`))
  (`/Game/Frigate/BP_PlayerCamera.SetSpringArm` _bp_playercamera (`self.SpringArm`))
  (`/Game/Frigate/BP_PlayerCamera.SetLengthRange` _bp_playercamera (`self.MinZoom`) (`self.MaxZoom`))
  (`/Game/Frigate/BP_PlayerCamera.SetLength` (`self.BP_PlayerCamera`) (`self.InitialZoom`)))